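; Game mode for DieselPunk that endlessly spawns timed waves of NPCs around the player, starting after BeginPlay.
; Two delayed waves alternate in a loop: small NPCs plus a middle one, then flying and small NPCs.
; Each spawn picks a random navigable point near player 0, raising flyers above it, and gives the NPC its default controller.
; Sequence pins repeat shared spawn chains, and the last branch loops back to the first delay.
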(event EventBeginPlay
  (Utilities|FlowControl|Sequence
    (:then_0
      (Utilities|FlowControl|Delay 25.0 :!label _label)
      (Utilities|FlowControl|Sequence
        (:then_0
          (bind _randomlocation (Class|NavigationSystemV1|GetRandomLocationinNavigableRadius (Transformation|GetActorLocation (Game|Player|GetPlayerPawn 0)) 7.5e+03 0 0 :!label _label_2))
          (bind _returnvalue (Game|SpawnActorfromClass "/Game/DieselPunk/Blueprints/Characters/BP_CharacterNPC_Small.BP_CharacterNPC_Small_C" (Math|Conversions|ToTransform(Vector) _randomlocation) "AdjustIfPossibleButAlwaysSpawn" "SelectDefaultAtRuntime" 0 0))
          (Utilities|IsValid _returnvalue
            (:Is%20Valid
              (Pawn|SpawnDefaultController _returnvalue))))
        (:then_1
          (goto _label_2))
        (:then_2
          (goto _label_2))
        (:then_3
          (goto _label_2))
        (:then_4
          (goto _label_2))
        (:then_5
          (goto _label_2))
        (:then_6
          (bind _randomlocation_2 (Class|NavigationSystemV1|GetRandomLocationinNavigableRadius (Transformation|GetActorLocation (Game|Player|GetPlayerPawn 0)) 7.5e+03 0 0))
          (bind _returnvalue_2 (Game|SpawnActorfromClass "/Game/DieselPunk/Blueprints/Characters/BP_CharacterNPC_Middle.BP_CharacterNPC_Middle_C" (Math|Conversions|ToTransform(Vector) _randomlocation_2) "AdjustIfPossibleButAlwaysSpawn" "SelectDefaultAtRuntime" 0 0))
          (Utilities|IsValid _returnvalue_2
            (:Is%20Valid
              (Pawn|SpawnDefaultController _returnvalue_2))))
        (:then_7
          (Utilities|FlowControl|Delay 25.0)
          (Utilities|FlowControl|Sequence
            (:then_0
              (bind _randomlocation_3 (Class|NavigationSystemV1|GetRandomLocationinNavigableRadius (Transformation|GetActorLocation (Game|Player|GetPlayerPawn 0)) 7.5e+03 0 0 :!label _label_3))
              (bind _returnvalue_3 (Game|SpawnActorfromClass "/Game/DieselPunk/Blueprints/Characters/BP_NPCFly.BP_NPCFly_C" (Math|Conversions|ToTransform(Vector) (Math|Vector|MakeVector (.x _randomlocation_3) (.y _randomlocation_3) (+ (.z _randomlocation_3) 5e+02))) "AdjustIfPossibleButAlwaysSpawn" "SelectDefaultAtRuntime" 0 0))
              (Utilities|IsValid _returnvalue_3
                (:Is%20Valid
                  (Pawn|SpawnDefaultController _returnvalue_3))))
            (:then_1
              (goto _label_3))
            (:then_2
              (goto _label_3))
            (:then_3
              (goto _label_3))
            (:then_4
              (goto _label_3))
            (:then_5
              (bind _randomlocation_4 (Class|NavigationSystemV1|GetRandomLocationinNavigableRadius (Transformation|GetActorLocation (Game|Player|GetPlayerPawn 0)) 7.5e+03 0 0 :!label _label_4))
              (bind _returnvalue_4 (Game|SpawnActorfromClass "/Game/DieselPunk/Blueprints/Characters/BP_CharacterNPC_Small.BP_CharacterNPC_Small_C" (Math|Conversions|ToTransform(Vector) _randomlocation_4) "AdjustIfPossibleButAlwaysSpawn" "SelectDefaultAtRuntime" 0 0))
              (Utilities|IsValid _returnvalue_4
                (:Is%20Valid
                  (Pawn|SpawnDefaultController _returnvalue_4))))
            (:then_6
              (goto _label_4))
            (:then_7
              (goto _label_4))
            (:then_8
              (goto _label_4))
            (:then_9
              (goto _label_4))
            (:then_10
              (goto _label_4))
            (:then_11
              (if true
                (goto _label)))))))))

(event EventTick
  (params (DeltaSeconds :type Float%20%28single-precision%29)))

(fn ConstructionScript)