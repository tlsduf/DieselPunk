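; BP_CharacterNPC_Small is a small NPC character Blueprint with minimal logic of its own.
; On BeginPlay it hides itself briefly, then reappears after a short delay.
; Each Tick it stores the capsule's yaw (Z) physics angular velocity in ActorRotationRate.
; Disconnected debug nodes for moving to the player and drawing navigation path points remain in the graph but never run.
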(event EventBeginPlay
  (Rendering|SetActorHiddenInGame true)
  (Utilities|FlowControl|Delay 0.4)
  (Rendering|SetActorHiddenInGame false))

(event Collision|EventActorBeginOverlap
  (params (OtherActor :type Actor%20Object%20Reference)))

(event EventTick
  (params (DeltaSeconds :type Float%20%28single-precision%29))
  (Variables|Default|SetActorRotationRate (.z (Physics|GetPhysicsAngularVelocityinDegrees (Variables|Default|GetCapsuleComponent) "None"))))

(event Game|Damage|EventAnyDamage
  (params (Damage :type Float%20%28single-precision%29) (DamageType :type Damage%20Type%20Object%20Reference) (InstigatedBy :type Controller%20Object%20Reference) (DamageCauser :type Actor%20Object%20Reference)))

(fn ConstructionScript)