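; NPC character Blueprint that manages the visibility of an overhead-style HP bar widget component.
; Any damage shows the bar and a retriggerable delay hides it after a quiet period, while Tick hides it whenever the character is dead.
; Tick also prints health percent to screen as debug output.
; Widget owner binding and an actor spawn sit in unconnected nodes that never run.
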(event EventBeginPlay)

(event Collision|EventActorBeginOverlap
  (params (OtherActor :type Actor%20Object%20Reference)))

(event EventTick
  (params (DeltaSeconds :type Float%20%28single-precision%29))
  (Utilities|FlowControl|Sequence
    (:then_0
      (if (Class|CharacterPC|IsDead)
        (Development|SetHiddeninGame (Variables|Default|GetHPBar) true false)))
    (:then_1
      (Development|PrintString (Utilities|String|ToString(Float) (Class|CharacterPC|GetHealthPercent)) true false "(R=0.000000,G=0.660000,B=1.000000,A=1.000000)" 0.0))))

(event Game|Damage|EventAnyDamage
  (params (Damage :type Float%20%28single-precision%29) (DamageType :type Damage%20Type%20Object%20Reference) (InstigatedBy :type Controller%20Object%20Reference) (DamageCauser :type Actor%20Object%20Reference))
  (Utilities|FlowControl|Sequence
    (:then_0
      (Development|SetHiddeninGame (Variables|Default|GetHPBar) false false)
      (Utilities|FlowControl|RetriggerableDelay 1e+01)
      (Development|SetHiddeninGame (Variables|Default|GetHPBar) true false))))

(fn ConstructionScript)