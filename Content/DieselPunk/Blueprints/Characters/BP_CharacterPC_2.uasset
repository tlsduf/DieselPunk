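; Player character Blueprint that adds rail grinding: landing on a component tagged "Rail" sends the character along that actor's spline.
; A Timeline moves the capsule in the direction matching its landing yaw, with play rate derived from remaining distance and speed bonus.
; Sprint raises the bonus and quiets the scrape sound.
; Jumping or reaching the end launches the character toward movement input, or forward, and restores collision, animation and effects.
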(event Custom|Stop%20Rail%20Timeline
  (bind _spline (Variables|Default|GetSpline))
  (bind _speedlines (Variables|Default|GetSpeedLines))
  (bind _spline_2 (Variables|Default|GetSpline))
  ;[1 1 1] The Timeline updates the position and rotation of the Character's Capsule above the Rail. When finished or when the Player inputs the Jump Button, the Timeline stops and the Jump from Rail Event triggers.
  (Utilities|FlowControl|Sequence
    (:then_0
      (bind _alpha (Timeline|Rail%20Timeline Stop)
        (:Update
          (Transformation|SetWorldLocationAndRotation (Variables|Default|GetCapsuleComponent) (+ (Spline|GetLocationatDistanceAlongSpline _spline (Math|Float|Lerp (Class|SplineComponent|GetDistanceAlongSplineatSplineInputKey _spline_2 (Class|SplineComponent|FindInputKeyClosesttoWorldLocation _spline_2 (Spline|FindLocationClosesttoWorldLocation _spline_2 (Variables|Default|GetHitLocation) "World"))) (Math|Float|SelectFloat (Spline|GetSplineLength (Variables|Default|GetSpline)) 0.0 (Variables|Default|GetForwardDirection)) _alpha) "World") "0, 0,120.000000") (Math|Rotator|MakeRotator 0.0 0.0 (select (Variables|Default|GetForwardDirection) (.yaw (Spline|GetRotationatDistanceAlongSpline _spline (Math|Float|Lerp (Class|SplineComponent|GetDistanceAlongSplineatSplineInputKey _spline_2 (Class|SplineComponent|FindInputKeyClosesttoWorldLocation _spline_2 (Spline|FindLocationClosesttoWorldLocation _spline_2 (Variables|Default|GetHitLocation) "World"))) (Math|Float|SelectFloat (Spline|GetSplineLength (Variables|Default|GetSpline)) 0.0 (Variables|Default|GetForwardDirection)) _alpha) "World")) (select (>= (Math|Rotator|NormalizeAxis (.yaw (Spline|GetRotationatDistanceAlongSpline _spline (Math|Float|Lerp (Class|SplineComponent|GetDistanceAlongSplineatSplineInputKey _spline_2 (Class|SplineComponent|FindInputKeyClosesttoWorldLocation _spline_2 (Spline|FindLocationClosesttoWorldLocation _spline_2 (Variables|Default|GetHitLocation) "World"))) (Math|Float|SelectFloat (Spline|GetSplineLength (Variables|Default|GetSpline)) 0.0 (Variables|Default|GetForwardDirection)) _alpha) "World"))) 0.0) (- (.yaw (Spline|GetRotationatDistanceAlongSpline _spline (Math|Float|Lerp (Class|SplineComponent|GetDistanceAlongSplineatSplineInputKey _spline_2 (Class|SplineComponent|FindInputKeyClosesttoWorldLocation _spline_2 (Spline|FindLocationClosesttoWorldLocation _spline_2 (Variables|Default|GetHitLocation) "World"))) (Math|Float|SelectFloat (Spline|GetSplineLength (Variables|Default|GetSpline)) 0.0 (Variables|Default|GetForwardDirection)) _alpha) "World")) 1.8e+02) (+ (.yaw (Spline|GetRotationatDistanceAlongSpline _spline (Math|Float|Lerp (Class|SplineComponent|GetDistanceAlongSplineatSplineInputKey _spline_2 (Class|SplineComponent|FindInputKeyClosesttoWorldLocation _spline_2 (Spline|FindLocationClosesttoWorldLocation _spline_2 (Variables|Default|GetHitLocation) "World"))) (Math|Float|SelectFloat (Spline|GetSplineLength (Variables|Default|GetSpline)) 0.0 (Variables|Default|GetForwardDirection)) _alpha) "World")) 1.8e+02)))) true false)
          ;[1 1 1] The relative Roll of the Skeletal Mesh is adjusted depending on the rotation of the Rail Spline. After the timeline finishes, the relative rotation of the Skeletal Mesh is set to normal. Also the rotation of the speedlines is adjusted here.
          (Transformation|SetRelativeRotation (Variables|Character|GetMesh) (Math|Rotator|MakeRotator 0.0 0.0 -9e+01) false false)
          (Utilities|IsValid _speedlines
            (:Is%20Valid
              (Transformation|SetRelativeRotation _speedlines (Math|Rotator|MakeRotator 0.0 0.0 0.0) false false))))
        (:Finished
          (CallFunction|JumpfromRail :!label _label))))
    (:then_1
      (goto _label))))

(event Custom|Stop%20Rail%20Sound%20FX
  ;[1 1 1] Animation when landing and particles + sound effects. We also update the SFX of the Rail if the Player is holding the Sprint Button, so its less louder and the footsteps can be heard.
  (Utilities|IsValid (stale EventOnLanded _returnvalue)
    (:Is%20Valid
      (Audio|Components|Audio|Stop (stale EventOnLanded _returnvalue)))))

(event Custom|Jump%20From%20Rail
  (bind _returnvalue (Pawn|GetControlRotation :!class /Script/Engine.Pawn))
  (bind _capsulecomponent (Variables|Default|GetCapsuleComponent))
  (bind _totalspeedbonus (Variables|Default|GetTotalSpeedBonus))
  (bind _minlaunchvelocity (Variables|Default|GetMinLaunchVelocity))
  (bind _maxlaunchvelocity (Variables|Default|GetMaxLaunchVelocity))
  (bind _moveforward (Variables|Default|GetMoveForward))
  (bind _moveright (Variables|Default|GetMoveRight))
  (bind _returnvalue_2 (Math|Vector|GetForwardVector _capsulecomponent))
  (bind _returnvalue_3 (Math|Float|MapRangeClamped _totalspeedbonus 0.0 1e+02 _minlaunchvelocity _maxlaunchvelocity))
  (bind _returnvalue_4 (Math|Vector|GetRightVector _returnvalue))
  (bind _returnvalue_5 (Math|Vector|GetForwardVector _returnvalue))
  (bind _returnvalue_6 (* _returnvalue_5 _moveforward))
  (bind _returnvalue_7 (* _returnvalue_4 _moveright))
  (bind _returnvalue_8 (+ _returnvalue_6 _returnvalue_7))
  ;[1 1 1] When jumping from the Rail, the character is launched depending on the resgistered directional input or if the Player is holding any directional input at all. If no directional input is registered, then the Character is Launched Forward. The Forward Vector X & Y is multiplied by a value that can be increased if you want the Character to be launched farther. In this example we have 500. The Launch Velocity Z is the upwards velocity, we have 550 in this case. The value can be increased to launch the Character higher.
  (if (and (== (Variables|Default|GetMoveForward) 0.0) (== (Variables|Default|GetMoveRight) 0.0))
    (Character|LaunchCharacter (Math|Vector|MakeVector (* (.x _returnvalue_2) 5e+02) (* (.y _returnvalue_2) 5e+02) 5.5e+02) true true)
    (else
      ;[1 1 1] Here we apply the same logic as above but the direction the Character is launched depends on the direction of the input. In the Map Range Clamped we take the value of Total Speed Bonus (the greater the value, the farther the Character will be launched). In the Min / Max Launch Velocity variables we can adjust how far. In the example we have 500 and 1000 as Min - Max. The same happens with the Launch Velocity Z. If you want a consistent launch velocity, regardless of Speed, then both Min and Max variables need to be the same.
      (Character|LaunchCharacter (Math|Vector|MakeVector (* (.x _returnvalue_8) _returnvalue_3) (* (.y _returnvalue_8) _returnvalue_3) (Math|Float|MapRangeClamped (Variables|Default|GetTotalSpeedBonus) 0.0 1e+02 (Variables|Default|GetMinUpwardsVelocity) (Variables|Default|GetMaxUpwardsVelocity))) true true)))
  (Variables|Default|SetSpline 0)
  ;[1 1 1] After jumping and clearing the reference to the Spline, we stop the Rail sound effect, detache and destroy the speedlines. If a Montage was playing, it is stopped. Sets the normal relative rotation of the Skeletal Mesh. After a short delay the character can move again and we set the Capsule collision to Block WorldStatic again
  (CallFunction|StopRailSoundFX)
  (Animation|StopAnimMontage 0)
  (Transformation|DetachFromComponent (Variables|Default|GetSpeedLines) "KeepWorld" "KeepWorld" "KeepWorld" true)
  (Components|DestroyComponent (Variables|Default|GetSpeedLines))
  (Variables|Default|SetSpeedLines 0)
  (bind _asmanny_anim_bp (Utilities|Casting|CastToManny_AnimBP (Components|SkeletalMesh|GetAnimInstance (Variables|Character|GetMesh)))
    (:then
      (Variables|/Game/SplineGrindRailBuilder/Demo/ThirdPersonAssets/Characters/Mannequins/Animations/Manny_AnimBP.Manny_AnimBP_C|SetIsInRail? _asmanny_anim_bp false))
    (:CastFailed
      _))
  (Transformation|SetRelativeRotation (Variables|Character|GetMesh) "0,-90.000000, 0" false false)
  (Utilities|FlowControl|Delay 0.1)
  (Variables|Default|SetCanMove true)
  (Collision|SetCollisionResponsetoChannel (Variables|Default|GetCapsuleComponent) "ECC_WorldStatic" "ECR_Block"))

(event Custom|Update%20Rail%20Sound%20FX
  ;[1 1 1] Animation when landing and particles + sound effects. We also update the SFX of the Rail if the Player is holding the Sprint Button, so its less louder and the footsteps can be heard.
  (Utilities|IsValid (stale EventOnLanded _returnvalue)
    (:Is%20Valid
      (Audio|Components|Audio|AdjustVolume (stale EventOnLanded _returnvalue) 0.25 (Math|Float|SelectFloat 0.15 1.0 (> (Class|PlayerController|GetInputKeyTimeDown (Game|GetPlayerController 0) (stale Input|ActionEvents|InputActionSprint Key)) 0.0)) "Linear" :!class /Script/Engine.AudioComponent))))

(event Input|EnhancedActionEvents|EnhancedInputActionIA_Space
  (params (ActionValue :type Boolean) (ElapsedSeconds :type Float%20%28double-precision%29) (TriggeredSeconds :type Float%20%28double-precision%29) (InputAction :type Input%20Action%20Object%20Reference :default "/Game/DieselPunk/Input/Actions/IA_Space.IA_Space"))
  ;[1 1 1] Jump: Before jumping we need to confirm that the Character is not in the Rail or able to move. If in Rail, it will stop the Timeline and launch the Character. If no Movement input is registered then the Character will be launched forward, but if there is Movement input registered then the Character will be launched in the direction of the input. Also, in the branch that checks if the Rail Timeline is Playing, you can add a boolean that checks if a Montage is Playing if you want to prevent the Character from being able to jump right after landing on the Rail.
  (:Started
    (if (Audio|Components|Audio|IsPlaying (Variables|Default|GetRail%20Timeline))
      (CallFunction|StopRailTimeline))))

(event EventOnLanded
  (params (Hit :type Hit%20Result%20Structure%20%28by%20ref%29))
  (bind (_bblockinghit _binitialoverlap _time _distance _location _impactpoint _normal _impactnormal _physmat _hitactor _hitcomponent) (Collision|BreakHitResult Hit))
  ;[1 1 1] Landing: we need to check if the character lands on the Rail by setting the variable 'Landed on Rail' to True if the Hit Component has the Tag 'Rail'. After that the rest of the logic will run.
  (Variables|Default|SetLandedOnRail (Components|ComponentHasTag _hitcomponent "Rail"))
  (Audio|PlaySoundatLocation 0 "0, 0, 0" "0, 0, 0" 1.0 1.0 0.0 0 0 0 0)
  (Effects|SpawnEmitteratLocation "/Game/SplineGrindRailBuilder/Particles/Smoke_PS.Smoke_PS" (- _location "0, 0,100.000000"))
  ;[1 1 1] The Character needs to land (and not just walk) above the Rail in order to set True the variable Landed on Rail. It saves the parameters used to calculate the direction of the character on the Rail and the Play Rate (Duration) of the Timeline. Here we also have the logic that sets the direction the Character should face when landing on the Rail (the variable Forward Direction). The variable Raw Rail Speed is the Speed on the Rail without the Total Speed Bonus. You can decrease the value of Raw Rail Speed Multiplier if you want the Character to move faster on Rails (what it does is setting how long it would take to travel a 1000 long Spline, in this example we have 0.6, so it would take 0.6 seconds to travel that distance, so if you change that for 0.4, it would travel 1000 in 0.4 seconds).
  (if (and (Variables|Default|GetLandedOnRail) (Variables|Default|GetCanMove))
    (Variables|Default|SetSpline (Actor|GetComponentbyClass _hitactor "/Script/Engine.SplineComponent"))
    (Variables|Default|SetRawRailSpeed (/ (* (Spline|GetSplineLength (Variables|Default|GetSpline)) (Variables|Default|GetRawRailSpeedMultiplier)) 1e+03))
    (Variables|Default|SetLandedOnRail false)
    (Variables|Default|SetCanMove false)
    (Variables|Default|SetHitLocation _impactpoint)
    (Variables|Default|SetForwardDirection (or (CallFunction|SimilarRotation? 9e+01) (CallFunction|SimilarRotation? -9e+01)))
    ;[1 1 1] Animation when landing and particles + sound effects. We also update the SFX of the Rail if the Player is holding the Sprint Button, so its less louder and the footsteps can be heard.
    (Utilities|FlowControl|Sequence
      (:then_0
        (Audio|PlaySoundatLocation "/Game/SplineGrindRailBuilder/Audio/Cues/Jumpland_Rail_Cue.Jumpland_Rail_Cue" "0, 0, 0" "0, 0, 0" 1.0 1.0 0.0 0 0 0 0)
        (bind _returnvalue (Audio|SpawnSoundatLocation "/Game/SplineGrindRailBuilder/Audio/Cues/Scrape_Cue.Scrape_Cue" "0, 0, 0" "0, 0, 0" 1.0 1.0 0.0 0 0))
        (CallFunction|UpdateRailSoundFX)
        (Animation|PlayAnimMontage 0 (Math|Float|MapRangeClamped (Variables|Default|GetTotalSpeedBonus) 0.0 1e+02 1.8 2.0) "None")
        ;[1 1 1] Sets the variable Is in Rail? to True inside the Character Animation Blueprint.
        (bind _asmanny_anim_bp (Utilities|Casting|CastToManny_AnimBP (Components|SkeletalMesh|GetAnimInstance (Variables|Character|GetMesh)))
          (:then
            (Variables|/Game/SplineGrindRailBuilder/Demo/ThirdPersonAssets/Characters/Mannequins/Animations/Manny_AnimBP.Manny_AnimBP_C|SetIsInRail? _asmanny_anim_bp true))
          (:CastFailed
            _))
        ;[1 1 1] Speedlines Niagara System parameters.
        (bind _returnvalue_2 (Niagara|SpawnSystemAttached "/Game/SplineGrindRailBuilder/NiagaraSystem/SpeedLines_NS.SpeedLines_NS" (Variables|Default|GetCapsuleComponent) "None" "0, 0,-40.000000" "0, 0, 0" "SnapToTarget" false true "None" false))
        (bind _output_get (Variables|Default|SetSpeedLines _returnvalue_2))
        (Niagara|SetNiagaraVariable(Float) _output_get "Lifetime Min" 0.4)
        (Niagara|SetNiagaraVariable(Float) _output_get "Lifetime Max" 0.8)
        ;[1 1 1] Here we calculate the Speed Without Bonus using the Raw Rail Speed to determine the final On Rail Speed (The Timeline Play Rate). Also we set the collision of the Character Capsule to only overlap WorldStatic so it doesn't collide with the Rail and can also grab coins. In the Function Update Timeline Play Rate we subtract the value of Total Speed Bonus (in percentage) from Speed Without Bonus to get the final On Rail Speed. The Total Speed Bonus value increases as the Player grabs green Bolts or holds the Input Sprint (Left Shift or Gamepad Face Button Left).
        (Variables|Default|SetSpeedWithoutBonus (Math|Float|SelectFloat (/ (* (Variables|Default|GetRawRailSpeed) (- (Spline|GetSplineLength (Variables|Default|GetSpline)) (Class|SplineComponent|GetDistanceAlongSplineatSplineInputKey (Variables|Default|GetSpline) (Class|SplineComponent|FindInputKeyClosesttoWorldLocation (Variables|Default|GetSpline) (Spline|FindLocationClosesttoWorldLocation (Variables|Default|GetSpline) (Variables|Default|GetHitLocation) "World"))))) (Spline|GetSplineLength (Variables|Default|GetSpline))) (/ (* (Variables|Default|GetRawRailSpeed) (Class|SplineComponent|GetDistanceAlongSplineatSplineInputKey (Variables|Default|GetSpline) (Class|SplineComponent|FindInputKeyClosesttoWorldLocation (Variables|Default|GetSpline) (Spline|FindLocationClosesttoWorldLocation (Variables|Default|GetSpline) (Variables|Default|GetHitLocation) "World")))) (Spline|GetSplineLength (Variables|Default|GetSpline))) (Variables|Default|GetForwardDirection)))
        (CallFunction|UpdateTimelinePlayRate)
        (Collision|SetCollisionResponsetoChannel (Variables|Default|GetCapsuleComponent) "ECC_WorldStatic" "ECR_Overlap")
        ;[1 1 1] The Timeline updates the position and rotation of the Character's Capsule above the Rail. When finished or when the Player inputs the Jump Button, the Timeline stops and the Jump from Rail Event triggers.
        (bind _alpha (Timeline|Rail%20Timeline PlayFromStart)
          (:Update
            (Transformation|SetWorldLocationAndRotation (Variables|Default|GetCapsuleComponent) (+ (Spline|GetLocationatDistanceAlongSpline (Variables|Default|GetSpline) (Math|Float|Lerp (Class|SplineComponent|GetDistanceAlongSplineatSplineInputKey (Variables|Default|GetSpline) (Class|SplineComponent|FindInputKeyClosesttoWorldLocation (Variables|Default|GetSpline) (Spline|FindLocationClosesttoWorldLocation (Variables|Default|GetSpline) (Variables|Default|GetHitLocation) "World"))) (Math|Float|SelectFloat (Spline|GetSplineLength (Variables|Default|GetSpline)) 0.0 (Variables|Default|GetForwardDirection)) _alpha) "World") "0, 0,120.000000") (Math|Rotator|MakeRotator 0.0 0.0 (select (Variables|Default|GetForwardDirection) (.yaw (Spline|GetRotationatDistanceAlongSpline (Variables|Default|GetSpline) (Math|Float|Lerp (Class|SplineComponent|GetDistanceAlongSplineatSplineInputKey (Variables|Default|GetSpline) (Class|SplineComponent|FindInputKeyClosesttoWorldLocation (Variables|Default|GetSpline) (Spline|FindLocationClosesttoWorldLocation (Variables|Default|GetSpline) (Variables|Default|GetHitLocation) "World"))) (Math|Float|SelectFloat (Spline|GetSplineLength (Variables|Default|GetSpline)) 0.0 (Variables|Default|GetForwardDirection)) _alpha) "World")) (select (>= (Math|Rotator|NormalizeAxis (.yaw (Spline|GetRotationatDistanceAlongSpline (Variables|Default|GetSpline) (Math|Float|Lerp (Class|SplineComponent|GetDistanceAlongSplineatSplineInputKey (Variables|Default|GetSpline) (Class|SplineComponent|FindInputKeyClosesttoWorldLocation (Variables|Default|GetSpline) (Spline|FindLocationClosesttoWorldLocation (Variables|Default|GetSpline) (Variables|Default|GetHitLocation) "World"))) (Math|Float|SelectFloat (Spline|GetSplineLength (Variables|Default|GetSpline)) 0.0 (Variables|Default|GetForwardDirection)) _alpha) "World"))) 0.0) (- (.yaw (Spline|GetRotationatDistanceAlongSpline (Variables|Default|GetSpline) (Math|Float|Lerp (Class|SplineComponent|GetDistanceAlongSplineatSplineInputKey (Variables|Default|GetSpline) (Class|SplineComponent|FindInputKeyClosesttoWorldLocation (Variables|Default|GetSpline) (Spline|FindLocationClosesttoWorldLocation (Variables|Default|GetSpline) (Variables|Default|GetHitLocation) "World"))) (Math|Float|SelectFloat (Spline|GetSplineLength (Variables|Default|GetSpline)) 0.0 (Variables|Default|GetForwardDirection)) _alpha) "World")) 1.8e+02) (+ (.yaw (Spline|GetRotationatDistanceAlongSpline (Variables|Default|GetSpline) (Math|Float|Lerp (Class|SplineComponent|GetDistanceAlongSplineatSplineInputKey (Variables|Default|GetSpline) (Class|SplineComponent|FindInputKeyClosesttoWorldLocation (Variables|Default|GetSpline) (Spline|FindLocationClosesttoWorldLocation (Variables|Default|GetSpline) (Variables|Default|GetHitLocation) "World"))) (Math|Float|SelectFloat (Spline|GetSplineLength (Variables|Default|GetSpline)) 0.0 (Variables|Default|GetForwardDirection)) _alpha) "World")) 1.8e+02)))) true false)
            ;[1 1 1] The relative Roll of the Skeletal Mesh is adjusted depending on the rotation of the Rail Spline. After the timeline finishes, the relative rotation of the Skeletal Mesh is set to normal. Also the rotation of the speedlines is adjusted here.
            (Transformation|SetRelativeRotation (Variables|Character|GetMesh) (Math|Rotator|MakeRotator 0.0 0.0 -9e+01) false false)
            (Utilities|IsValid (Variables|Default|GetSpeedLines)
              (:Is%20Valid
                (Transformation|SetRelativeRotation (Variables|Default|GetSpeedLines) (Math|Rotator|MakeRotator 0.0 0.0 0.0) false false))))
          (:Finished
            (CallFunction|JumpfromRail))))
      (:then_1
        (Effects|SpawnEmitteratLocation "/Game/SplineGrindRailBuilder/Particles/Sparks_PS.Sparks_PS" (- (Transformation|GetWorldLocation (Variables|Default|GetCapsuleComponent)) "0, 0,95.000000") :!label _label)
        (Utilities|FlowControl|Delay 0.1)
        (if (Audio|Components|Audio|IsPlaying (Variables|Default|GetRail%20Timeline))
          (goto _label))))))

(event Input|ActionEvents|InputActionSprint
  (params (Key :type Key%20Structure :default "None"))
  (bind _returnvalue (Game|GetPlayerController 0))
  (bind _returnvalue_2 (Class|PlayerController|GetInputKeyTimeDown _returnvalue Key))
  (bind _returnvalue_3 (> _returnvalue_2 0.0))
  ;[1 1 1] Sprint on Rails: Holding the Button (Left Shift or Gamepad Face Button Left) will make the Character Sprint on Rails. The Total Speed Bonus will increase by 5% and decrease by 5% when releasing the Button. You can change that value here. The Timeline Play Rate will be updated to reflect the Speed boost.
  (:Pressed
    (Utilities|IsValid _returnvalue :!label _label
      (:Is%20Valid
        (bind _asmanny_anim_bp (Utilities|Casting|CastToManny_AnimBP (Components|SkeletalMesh|GetAnimInstance (Variables|Character|GetMesh))))
        (Variables|/Game/SplineGrindRailBuilder/Demo/ThirdPersonAssets/Characters/Mannequins/Animations/Manny_AnimBP.Manny_AnimBP_C|SetSprint? _asmanny_anim_bp _returnvalue_3)
        (Variables|Default|SetTotalSpeedBonus (+ (Variables|Default|GetTotalSpeedBonus) (Math|Float|SelectFloat 5.0 -5.0 _returnvalue_3)))
        (if (Audio|Components|Audio|IsPlaying (Variables|Default|GetRail%20Timeline))
          (CallFunction|UpdateTimelinePlayRate)
          (CallFunction|UpdateRailSoundFX)))))
  (:Released
    (goto _label)))

(fn ConstructionScript)

(fn SimilarRotation?
  (params (Z%20Var :type Float%20%28double-precision%29))
  (bind _spline (Variables|Default|GetSpline))
  (bind _capsulecomponent (Variables|Default|GetCapsuleComponent))
  (bind _hitlocation (Variables|Default|GetHitLocation))
  (bind _returnvalue (Spline|FindLocationClosesttoWorldLocation _spline _hitlocation "World"))
  (bind _returnvalue_2 (Transformation|GetWorldRotation _capsulecomponent))
  (bind _returnvalue_3 (Class|SplineComponent|FindInputKeyClosesttoWorldLocation _spline _returnvalue))
  (bind _returnvalue_4 (Class|SplineComponent|GetDistanceAlongSplineatSplineInputKey _spline _returnvalue_3))
  (bind _returnvalue_5 (Spline|GetRotationatDistanceAlongSpline _spline _returnvalue_4 "World"))
  (bind _returnvalue_6 (+ (.yaw _returnvalue_5) Z%20Var))
  (bind _returnvalue_7 (Math|Rotator|NormalizeAxis _returnvalue_6))
  (bind _returnvalue_8 (Math|Float|NearlyEqual(Float) _returnvalue_6 _returnvalue_7 0.1))
  (bind _returnvalue_9 (> (.yaw _returnvalue_5) _returnvalue_7))
  (bind _returnvalue_10 (Math|Float|SelectFloat (.yaw _returnvalue_5) _returnvalue_7 _returnvalue_9))
  (bind _returnvalue_11 (Math|Float|SelectFloat _returnvalue_7 (.yaw _returnvalue_5) _returnvalue_9))
  (bind _returnvalue_12 (select _returnvalue_8 true false))
  (bind _returnvalue_13 (Math|Float|InRange(Float) (.yaw _returnvalue_2) _returnvalue_11 _returnvalue_10 _returnvalue_12 _returnvalue_12))
  (return (select _returnvalue_8 _returnvalue_13 (not _returnvalue_13))))

(fn UpdateTimelinePlayRate
  (Variables|Default|SetOnRailSpeed (- (Variables|Default|GetSpeedWithoutBonus) (/ (* (Variables|Default|GetSpeedWithoutBonus) (Variables|Default|GetTotalSpeedBonus)) 1e+02)))
  (Components|Timeline|SetPlayRate (Variables|Default|GetRail%20Timeline) (/ 1.0 (Math|Float|SelectFloat 0.1 (Variables|Default|GetOnRailSpeed) (<= (Variables|Default|GetOnRailSpeed) 0.0)))))