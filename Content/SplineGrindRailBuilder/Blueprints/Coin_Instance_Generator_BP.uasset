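; Coin instance generator that renders every Coin_BP in the level through one Hierarchical Instanced Static Mesh instead of a mesh per coin.
; The Construction Script gathers all Coin_BP actors and adds an instance at each location with random yaw.
; The GrabCoin interface event line-traces vertically through the given coin location and removes the hit instance by its HitItem index.
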(event EventGrabCoin
  (params (CoinLocation :type Vector :default "0, 0, 0"))
  ;[1 1 1 1 20] This Blueprint implements the Coin Interface BP so every time the Character collides with a Coin BP, its location is sent here so a Line Trace is used to get the Coin instance index and remove that instance. In this project, getting Coins doesn't affect gameplay, only green Bolts do by increasing Speed. You can use Coins to increase a Score or change the mesh to another object and apply a custom functionality.
  (bind (_outhit _returnvalue) (Collision|LineTraceByChannel (+ CoinLocation "0, 0,50.000000") (- CoinLocation "0, 0,50.000000") "TraceTypeQuery1" false 0 "None" false))
  (if _returnvalue
    (Class|InstancedStaticMeshComponent|RemoveInstance (Variables|Default|GetCoin) (.HitItem (Collision|BreakHitResult _outhit)))))

(fn ConstructionScript
  ;[1 1 1 1 20] To avoid adding 1 Coin mesh per Coin BP, we use this Blueprint to create instances of the Coin at the location of every Coin BP in the Level.
  (bind _returnvalue (AddComponent|AddHierarchicalInstancedStaticMeshComponent false))
  (Variables|Default|SetCoin _returnvalue)
  (bind _outactors (Actor|GetAllActorsOfClass "/Game/SplineGrindRailBuilder/Blueprints/Coin_BP.Coin_BP_C"))
  (for _array_element _outactors
    (Components|InstancedStaticMesh|AddInstance (Variables|Default|GetCoin) (Math|Transform|MakeTransform (Transformation|GetActorLocation _array_element) (Math|Rotator|MakeRotator 0.0 0.0 (Math|Random|RandomFloatinRange 0.0 1.8e+02)) "1.000000,1.000000,1.000000") false)))