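; Spline-based rail actor that builds a mesh rail, tagged "Rail", along its spline in the construction script, with optional supports.
; Each spline segment becomes a spline mesh with query-only collision that ignores the camera channel.
; Supports sit at percentages of spline length: either or both ends, inset by total length, plus up to four intermediates.
; Each support traces down to the floor, scales an instanced mesh to that height, and adds height-dependent base meshes.
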(fn ConstructionScript
  (bind _spline (Variables|Default|GetSpline))
  (bind _spline_2 (Variables|Default|GetSpline))
  (bind _returnvalue (Spline|GetSplineLength _spline))
  (bind _returnvalue_2 (Math|Float|MapRangeClamped _returnvalue 5e+02 7e+03 7.5 0.75))
  (bind _returnvalue_3 (Math|Float|MapRangeClamped _returnvalue 7e+03 5e+02 99.25 92.5))
  (for _index (range 0 (- (Spline|GetNumberOfSplinePoints _spline_2) 2))
    (bind _returnvalue_4 (AddComponent|AddSplineMeshComponent false))
    (Variables|/Script/Engine.ActorComponent|SetComponentTags _returnvalue_4 (Utilities|Array|MakeArray "Rail"))
    (Components|StaticMesh|SetStaticMesh _returnvalue_4 (Variables|Default|GetSplineMesh))
    (SplineMesh|SetForwardAxis _returnvalue_4 (Variables|Default|GetForward%20Axis) true)
    (Transformation|AttachComponentToComponent _returnvalue_4 _spline_2 "None" "KeepRelative" "KeepRelative" "KeepRelative" true)
    (SplineMesh|SetStartandEnd _returnvalue_4 (Spline|GetLocationatSplinePoint _spline_2 _index "Local") (Spline|GetTangentatSplinePoint _spline_2 _index "Local") (Spline|GetLocationatSplinePoint _spline_2 (+ _index 1) "Local") (Spline|GetTangentatSplinePoint _spline_2 (+ _index 1) "Local") true :!class /Script/Engine.SplineMeshComponent)
    (Collision|SetCollisionProfileName _returnvalue_4 "BlockAll" true :!class /Script/Engine.PrimitiveComponent)
    (Collision|SetCollisionEnabled _returnvalue_4 "QueryOnly")
    (Collision|SetCollisionObjectType _returnvalue_4 "ECC_WorldStatic")
    (Collision|SetCollisionResponsetoChannel _returnvalue_4 "ECC_Camera" "ECR_Ignore")
    (Rendering|Material|SetMaterial _returnvalue_4 0 (Variables|Default|GetSplineMeshMaterial))
    (Variables|/Script/Engine.PrimitiveComponent|SetbGenerateOverlapEvents _returnvalue_4 false))
  ;[1 1 1 1 20] This Function uses a Float to determine the location of a point in the Spline's Length based on a percentage (for example, 5.0 is 5 % of the lenght of the Spline so a support will be added at that location).
  (if (Variables|Default|GetCreateSupports?)
    (switch Utilities|FlowControl|Switch|SwitchonRailSupport_Enum (Variables|Default|GetRailSupportLocation)
      (:NewEnumerator0
        (CallFunction|CreateSupports _returnvalue_2)
        (CallFunction|CreateSupports _returnvalue_3))
      (:NewEnumerator1
        (CallFunction|CreateSupports _returnvalue_2))
      (:NewEnumerator2
        (CallFunction|CreateSupports _returnvalue_3)))
    (if (Variables|Default|GetCreateAdditionalSupports?)
      (switch int (Variables|Default|GetQuantityOfAdditionalSupports)
        (:1
          (CallFunction|CreateSupports 5e+01))
        (:2
          (CallFunction|CreateSupports 35.0)
          (CallFunction|CreateSupports 65.0))
        (:3
          (CallFunction|CreateSupports 27.5)
          (CallFunction|CreateSupports 5e+01)
          (CallFunction|CreateSupports 72.5))
        (:4
          (CallFunction|CreateSupports 23.0)
          (CallFunction|CreateSupports 41.0)
          (CallFunction|CreateSupports 59.0)
          (CallFunction|CreateSupports 77.0))))))

(fn CreateSupports
  (params (LocationBasedOnSpline'sLenghtPercentage :type Float%20%28double-precision%29))
  ;[1 1 1 1 20] Here, we add an Instance of a Mesh for the Rail Support. It calculates the distance to the floor and adds the Instance with a varied Z Scale to match the height. You can change the Support Mesh here. In this example we are using a cylinder and apply the same material of the Spline Mesh.
  (bind _returnvalue (AddComponent|AddHierarchicalInstancedStaticMeshComponent false))
  (Rendering|Material|SetMaterial _returnvalue 0 (Variables|Default|GetSplineMeshMaterial))
  (Variables|Default|SetDistanceAlongSpline (/ (* (Spline|GetSplineLength (Variables|Default|GetSpline)) LocationBasedOnSpline'sLenghtPercentage) 1e+02))
  (bind (_outhit _returnvalue_2) (Collision|LineTraceByChannel (Spline|GetLocationatDistanceAlongSpline (Variables|Default|GetSpline) (Variables|Default|GetDistanceAlongSpline) "World") (- (Spline|GetLocationatDistanceAlongSpline (Variables|Default|GetSpline) (Variables|Default|GetDistanceAlongSpline) "World") "0, 0,100000.000000") "TraceTypeQuery1" false 0 "None"))
  (if _returnvalue_2
    (Variables|Default|SetDistance (.Distance (Collision|BreakHitResult _outhit)))
    (Variables|Default|SetSupportBaseLocation (- (Spline|GetLocationatDistanceAlongSpline (Variables|Default|GetSpline) (Variables|Default|GetDistanceAlongSpline) "Local") (Math|Vector|MakeVector 0.0 0.0 (Variables|Default|GetDistance))))
    (Components|InstancedStaticMesh|AddInstance _returnvalue (Math|Transform|MakeTransform (Variables|Default|GetSupportBaseLocation) "0, 0, 0" (Math|Vector|MakeVector 1.0 1.0 (* (/ (Variables|Default|GetDistance) 2e+02) 1.0))) false)
    ;[1 1 1 1 20] Here we add a Base Mesh Instance for the Support Mesh. It varies depending on the height. You can also change the Mesh here and the Materials.
    (if (> (Variables|Default|GetDistance) 2e+01)
      (bind _returnvalue_3 (AddComponent|AddHierarchicalInstancedStaticMeshComponent false))
      (Rendering|Material|SetMaterial _returnvalue_3 0 (Variables|Default|GetSupportMeshMaterial))
      (if (< (Variables|Default|GetDistance) 85.0)
        (if (< (Variables|Default|GetDistance) 5e+01)
          (Components|InstancedStaticMesh|AddInstance _returnvalue_3 (Math|Transform|MakeTransform (Variables|Default|GetSupportBaseLocation) "0, 0, 0" (Math|Vector|MakeVector 1.2 1.2 (Math|Float|SelectFloat (/ (* (/ (Variables|Default|GetDistance) 2e+02) 1.0) 4.0) 0.25 (< (Variables|Default|GetDistance) 1e+02)))) false)
          (else
            (bind _returnvalue_4 (AddComponent|AddHierarchicalInstancedStaticMeshComponent false :!label _label))
            (Rendering|Material|SetMaterial _returnvalue_4 0 (Variables|Default|GetSupportMeshMaterial))
            (Components|InstancedStaticMesh|AddInstance _returnvalue_4 (Math|Transform|MakeTransform (Variables|Default|GetSupportBaseLocation) (Math|Rotator|MakeRotator 0.0 0.0 (.Yaw (Math|Rotator|BreakRotator (Spline|GetRotationatDistanceAlongSpline (Variables|Default|GetSpline) (Variables|Default|GetDistanceAlongSpline) "Local")))) "1.000000,1.000000,1.000000") false)
            (Components|InstancedStaticMesh|AddInstance _returnvalue_3 (Math|Transform|MakeTransform (Variables|Default|GetSupportBaseLocation) "0, 0, 0" "1.600000,1.600000,0.100000") false)))
        (else
          (Components|InstancedStaticMesh|AddInstance _returnvalue_3 (Math|Transform|MakeTransform (Variables|Default|GetSupportBaseLocation) "0, 0, 0" "1.200000,1.200000,0.250000") false)
          (goto _label))))))