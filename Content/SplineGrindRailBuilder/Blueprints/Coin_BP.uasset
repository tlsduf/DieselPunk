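; Collectible coin actor that the player picks up by overlapping its sphere.
; The construction script caches the Coin_Instance_Generator_BP found in the level.
; On overlap it disables collision, hides itself and sends its location to that generator through GrabCoinMessage, so the matching coin instance can be removed.
; It also deactivates its particle, spawns a pickup spark effect at the coin and plays the grab sound at world origin.
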(event OnComponentBeginOverlap(Sphere)
  (params (OverlappedComponent :type Primitive%20Component%20Object%20Reference) (OtherActor :type Actor%20Object%20Reference) (OtherComp :type Primitive%20Component%20Object%20Reference) (OtherBodyIndex :type Integer) (bFromSweep :type Boolean) (SweepResult :type Hit%20Result%20Structure%20%28by%20ref%29))
  (bind _returnvalue (Transformation|GetActorLocation))
  ;[1 1 1 1 20] Each time the Player touches a Coin, this Blueprint sends its location to the Coin Instance Generator BP, so that blueprint can remove the Coin Instance at that location. A sound FX is fired and a Particle System spawns. Then this Actor is set hidden and its collision disabled.
  (Collision|SetActorEnableCollision false)
  (Rendering|SetActorHiddenInGame true)
  (Components|Activation|Deactivate (Variables|Default|GetParticle))
  (Class|CoinInterfaceBP|GrabCoin(Message) (Variables|Default|GetCoinInstanceGenerator) _returnvalue)
  (Effects|SpawnEmitteratLocation "/Game/SplineGrindRailBuilder/Particles/Sparks_Pickup_PS.Sparks_Pickup_PS" _returnvalue)
  (Audio|PlaySoundatLocation "/Game/SplineGrindRailBuilder/Audio/Cues/Grab_Coin_Cue.Grab_Coin_Cue" "0, 0, 0" "0, 0, 0" 1.0 1.0 0.0 0 0 0 0))

(fn ConstructionScript
  (bind _returnvalue (Actor|GetActorOfClass "/Game/SplineGrindRailBuilder/Blueprints/Coin_Instance_Generator_BP.Coin_Instance_Generator_BP_C"))
  (Variables|Default|SetCoinInstanceGenerator _returnvalue))