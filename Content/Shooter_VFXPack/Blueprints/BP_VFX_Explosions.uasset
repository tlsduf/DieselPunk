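; Explosion VFX actor that spawns a Niagara effect at its transform after a start delay and repeats it on a delayed loop.
; Each blast traces downward and places a BP_DecalExplosion on the surface, sized and timed by ExplosionType.
; With BigExplosion set, it also scatters small explosions and decals at random navmesh points, with randomized delays that grow with distance to stagger them outward.
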(event Custom|Again
  (bind _returnvalue (Transformation|GetActorLocation))
  (bind _returnvalue_2 (Transformation|GetActorTransform))
  (bind _returnvalue_3 (Transformation|GetActorLocation))
  (bind _returnvalue_4 (Math|Random|RandomFloatinRange 0.3 0.5))
  (bind (_randomlocation _returnvalue_5) (Class|NavigationSystemV1|GetRandomPointinNavigableRadius _returnvalue_3 8e+02 0 0))
  (Utilities|FlowControl|Delay (Variables|Default|GetDelay))
  (Niagara|SpawnSystematLocation (Variables|Default|GetEffect) (.location _returnvalue_2) (.rotation _returnvalue_2))
  (CallFunction|Again)
  (Utilities|FlowControl|Sequence
    (:then_0
      ;[1 1 1] Big Explosion
      (if (Variables|Default|GetBigExplosion)
        (Variables|Default|SetExp 0.0)
        (while (< (Variables|Default|GetExp) 25.0)
          (if _returnvalue_5
            (bind _returnvalue_6 (Niagara|SpawnSystematLocation (Variables|Default|GetSmallExplosions) _randomlocation))
            (bind _output_get (Variables|Default|SetDecalDelay (+ (Math|Random|RandomFloatinRange 0.1 0.5) (+ (* (Math|Vector|Distance(Vector) (Transformation|GetWorldLocation _returnvalue_6) (Transformation|GetActorLocation)) 0.0005) 0.0))))
            (Effects|Components|ParticleSystem|SetFloatParameter _returnvalue_6 "User.Delay" _output_get)
            (Effects|Components|ParticleSystem|SetBoolParameter _returnvalue_6 "User.Circle" false)
            (Effects|Components|ParticleSystem|SetFloatParameter _returnvalue_6 "User.Radius" (Math|Random|RandomFloatinRange 1.1e+02 2.2e+02))
            (Math|Float|IncrementFloat (Variables|Default|GetExp)
              (:%20%20
                (Game|SpawnActorfromClass "/Game/Shooter_VFXPack/Blueprints/BP_DecalExplosion.BP_DecalExplosion_C" (Math|Transform|MakeTransform (Transformation|GetWorldLocation _returnvalue_6) "0, 0, 0" (Math|Vector|MakeVector 1.0 _returnvalue_4 _returnvalue_4)) "Undefined" 0 1 1.5 0.5 false (+ (Variables|Default|GetDecalDelay) 0.1) 0)))
            (else
              (Math|Float|IncrementFloat (Variables|Default|GetExp)))))))
    (:then_1
      (bind (_outhit _returnvalue_7) (Collision|LineTraceByChannel _returnvalue (+ _returnvalue "0, 0,-500.000000") "TraceTypeQuery1" false 0 "None"))
      (if _returnvalue_7
        (switch int (Variables|Default|GetExplosionType)
          (:0
            (Game|SpawnActorfromClass "/Game/Shooter_VFXPack/Blueprints/BP_DecalExplosion.BP_DecalExplosion_C" (Math|Transform|MakeTransform (.ImpactPoint (Collision|BreakHitResult _outhit)) (Math|Rotator|MakeRotfromZ (.ImpactNormal (Collision|BreakHitResult _outhit))) "1,0.150000,0.150000") "Undefined" 0 0 2.0 1.5 false 0.1 0))
          (:1
            (Game|SpawnActorfromClass "/Game/Shooter_VFXPack/Blueprints/BP_DecalExplosion.BP_DecalExplosion_C" (Math|Transform|MakeTransform (.ImpactPoint (Collision|BreakHitResult _outhit)) (Math|Rotator|MakeRotfromZ (.ImpactNormal (Collision|BreakHitResult _outhit))) "1,0.500000,0.500000") "Undefined" 0 1 2.0 1.5 false 0.1 0))
          (:2
            (Game|SpawnActorfromClass "/Game/Shooter_VFXPack/Blueprints/BP_DecalExplosion.BP_DecalExplosion_C" (Math|Transform|MakeTransform (.ImpactPoint (Collision|BreakHitResult _outhit)) (Math|Rotator|MakeRotfromZ (.ImpactNormal (Collision|BreakHitResult _outhit))) "1,0.700000,0.700000") "Undefined" 0 2 4.0 0.5 false 0.1 0))
          (:3
            (Game|SpawnActorfromClass "/Game/Shooter_VFXPack/Blueprints/BP_DecalExplosion.BP_DecalExplosion_C" (Math|Transform|MakeTransform (.ImpactPoint (Collision|BreakHitResult _outhit)) (Math|Rotator|MakeRotfromZ (.ImpactNormal (Collision|BreakHitResult _outhit))) "1,1,1") "Undefined" 0 3 4.0 0.5 false 0.1 0)))))))

(event EventBeginPlay
  (bind _returnvalue (Transformation|GetActorLocation))
  (bind _returnvalue_2 (Transformation|GetActorTransform))
  (bind _returnvalue_3 (Transformation|GetActorLocation))
  (bind _returnvalue_4 (Math|Random|RandomFloatinRange 0.3 0.5))
  (bind (_randomlocation _returnvalue_5) (Class|NavigationSystemV1|GetRandomPointinNavigableRadius _returnvalue_3 8e+02 0 0))
  (Utilities|FlowControl|Delay (Variables|Default|GetStart_Delay))
  (Niagara|SpawnSystematLocation (Variables|Default|GetEffect) (.location _returnvalue_2) (.rotation _returnvalue_2))
  (CallFunction|Again)
  (Utilities|FlowControl|Sequence
    (:then_0
      ;[1 1 1] Big Explosion
      (if (Variables|Default|GetBigExplosion)
        (Variables|Default|SetExp 0.0)
        (while (< (Variables|Default|GetExp) 25.0)
          (if _returnvalue_5
            (bind _returnvalue_6 (Niagara|SpawnSystematLocation (Variables|Default|GetSmallExplosions) _randomlocation))
            (bind _output_get (Variables|Default|SetDecalDelay (+ (Math|Random|RandomFloatinRange 0.1 0.5) (+ (* (Math|Vector|Distance(Vector) (Transformation|GetWorldLocation _returnvalue_6) (Transformation|GetActorLocation)) 0.0005) 0.0))))
            (Effects|Components|ParticleSystem|SetFloatParameter _returnvalue_6 "User.Delay" _output_get)
            (Effects|Components|ParticleSystem|SetBoolParameter _returnvalue_6 "User.Circle" false)
            (Effects|Components|ParticleSystem|SetFloatParameter _returnvalue_6 "User.Radius" (Math|Random|RandomFloatinRange 1.1e+02 2.2e+02))
            (Math|Float|IncrementFloat (Variables|Default|GetExp)
              (:%20%20
                (Game|SpawnActorfromClass "/Game/Shooter_VFXPack/Blueprints/BP_DecalExplosion.BP_DecalExplosion_C" (Math|Transform|MakeTransform (Transformation|GetWorldLocation _returnvalue_6) "0, 0, 0" (Math|Vector|MakeVector 1.0 _returnvalue_4 _returnvalue_4)) "Undefined" 0 1 1.5 0.5 false (+ (Variables|Default|GetDecalDelay) 0.1) 0)))
            (else
              (Math|Float|IncrementFloat (Variables|Default|GetExp)))))))
    (:then_1
      (bind (_outhit _returnvalue_7) (Collision|LineTraceByChannel _returnvalue (+ _returnvalue "0, 0,-500.000000") "TraceTypeQuery1" false 0 "None"))
      (if _returnvalue_7
        (switch int (Variables|Default|GetExplosionType)
          (:0
            (Game|SpawnActorfromClass "/Game/Shooter_VFXPack/Blueprints/BP_DecalExplosion.BP_DecalExplosion_C" (Math|Transform|MakeTransform (.ImpactPoint (Collision|BreakHitResult _outhit)) (Math|Rotator|MakeRotfromZ (.ImpactNormal (Collision|BreakHitResult _outhit))) "1,0.150000,0.150000") "Undefined" 0 0 2.0 1.5 false 0.1 0))
          (:1
            (Game|SpawnActorfromClass "/Game/Shooter_VFXPack/Blueprints/BP_DecalExplosion.BP_DecalExplosion_C" (Math|Transform|MakeTransform (.ImpactPoint (Collision|BreakHitResult _outhit)) (Math|Rotator|MakeRotfromZ (.ImpactNormal (Collision|BreakHitResult _outhit))) "1,0.500000,0.500000") "Undefined" 0 1 2.0 1.5 false 0.1 0))
          (:2
            (Game|SpawnActorfromClass "/Game/Shooter_VFXPack/Blueprints/BP_DecalExplosion.BP_DecalExplosion_C" (Math|Transform|MakeTransform (.ImpactPoint (Collision|BreakHitResult _outhit)) (Math|Rotator|MakeRotfromZ (.ImpactNormal (Collision|BreakHitResult _outhit))) "1,0.700000,0.700000") "Undefined" 0 2 4.0 0.5 false 0.1 0))
          (:3
            (Game|SpawnActorfromClass "/Game/Shooter_VFXPack/Blueprints/BP_DecalExplosion.BP_DecalExplosion_C" (Math|Transform|MakeTransform (.ImpactPoint (Collision|BreakHitResult _outhit)) (Math|Rotator|MakeRotfromZ (.ImpactNormal (Collision|BreakHitResult _outhit))) "1,1,1") "Undefined" 0 3 4.0 0.5 false 0.1 0)))))))

(fn ConstructionScript)