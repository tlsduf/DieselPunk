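; Classic VFX projectile with a Niagara trail, optional gravity and a configurable initial speed that is also fed to the trail.
; Each tick it line-traces ahead along its forward vector, scaled by speed and frame time, to detect impacts before reaching them.
; On a hit it snaps the trail to the impact, optionally spawns a hit effect, plus a decal when normal-aligned, then stops and self-destructs after a delay.
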(event EventBeginPlay
  (Class|NiagaraComponent|SetAsset (Variables|Default|GetTrail) (Variables|Default|GetNiagara_Trail) true)
  (Variables|/Script/Engine.ProjectileMovementComponent|SetProjectileGravityScale (Variables|Default|GetProjectileMovement) (Math|Conversions|ToFloat(Boolean) (Variables|Default|GetbGravity%20Enabled))))

(event EventTick
  (params (DeltaSeconds :type Float%20%28single-precision%29))
  (bind _returnvalue (Transformation|GetActorLocation))
  (bind _hiteffect (Variables|Default|GetHitEffect))
  (if (not (Variables|Default|GetbHitOK))
    (bind (_outhit _returnvalue_2) (Collision|LineTraceByChannel _returnvalue (+ _returnvalue (* (Transformation|GetActorForwardVector) (* (Variables|Default|GetInitial%20Speed) (* (Utilities|Time|GetWorldDeltaSeconds) 1.3)))) "TraceTypeQuery1" false 0 "None" true "(R=1.000000,G=0.000000,B=0.000000,A=1.000000)" "(R=0.000000,G=1.000000,B=0.000000,A=1.000000)" 0.1))
    (if _returnvalue_2
      (Variables|Default|SetbHitOK true)
      (Effects|Components|ParticleSystem|SetBoolParameter (Variables|Default|GetTrail) "User.SpawnLastParticle" true)
      (Utilities|FlowControl|Delay 0.0)
      (Transformation|SetWorldLocation (Variables|Default|GetTrail) (.ImpactPoint (Collision|BreakHitResult _outhit)) false false)
      (Utilities|FlowControl|Sequence
        (:then_0
          (Utilities|FlowControl|Delay 0.0)
          (Components|Activation|Deactivate (Variables|Default|GetTrail))
          (Components|Movement|StopMovementImmediately (Variables|Default|GetProjectileMovement))
          (Collision|SetCollisionEnabled (Variables|Default|GetSphere) "NoCollision")
          (Utilities|FlowControl|Delay 5.0)
          (Actor|DestroyActor))
        (:then_1
          (if (Variables|Default|GetbHit)
            (if (Variables|Default|GetbImpactNormal)
              (Niagara|SpawnSystematLocation _hiteffect (.ImpactPoint (Collision|BreakHitResult _outhit)) (Math|Rotator|MakeRotfromX (.ImpactNormal (Collision|BreakHitResult _outhit))))
              (Game|SpawnActorfromClass "/Game/Shooter_VFXPack/Blueprints/BP_DecalHit.BP_DecalHit_C" (Math|Transform|MakeTransform (.ImpactPoint (Collision|BreakHitResult _outhit)) (Math|Rotator|MakeRotfromZ (.ImpactNormal (Collision|BreakHitResult _outhit))) (Math|Conversions|ToVector(Float) (Math|Random|RandomFloatinRange 0.6 0.95))) "Undefined" 0 1.5 1.0 false 0.0 (Variables|Default|GetEmissive%20Color) 0)
              (else
                (Niagara|SpawnSystematLocation _hiteffect (.ImpactPoint (Collision|BreakHitResult _outhit)) (Math|Rotator|MakeRotfromX (- (.TraceStart (Collision|BreakHitResult _outhit)) (.ImpactPoint (Collision|BreakHitResult _outhit)))))))))))))

(fn ConstructionScript
  (bind _initial_speed (Variables|Default|GetInitial%20Speed))
  (Variables|/Script/Engine.ProjectileMovementComponent|SetInitialSpeed (Variables|Default|GetProjectileMovement) _initial_speed)
  (Effects|Components|ParticleSystem|SetFloatParameter (Variables|Default|GetTrail) "User.ProjSpeed" _initial_speed))